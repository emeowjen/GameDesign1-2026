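; Stealth-game enemy that patrols, spots the player through PawnSensing and gives chase, with debug prints as reactions.
; Tick chooses between chasing, looping through target points or wandering to random reachable points, using a CanMove flag to gate patrol moves.
; Chasing overrides that gate and raises walk speed, while patrols lower it.
; Each sighting restarts a retriggerable delay that clears PlayerVisible once the player stays unseen briefly.
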(event `self.ReceiveBeginPlay`)

(event `self.ReceiveTick`
  (params (DeltaSeconds :type "Float (single-precision)"))
  (bind _bplayervisible (`self.bPlayerVisible`))
  (if (`self.bCanMove`)
    (if _bplayervisible
      (`self.ChasePlayer`)
      (elif (`self.bTargetPointBoolean`)
        (`self.MoveToNextPatrolPoint`)
        (else
          (`self.PatrolRandom`))))
    (elif _bplayervisible
      (`self.ChasePlayer`))))

(event `self.PawnSensing.OnSeePawn`
  (params (Pawn :type "Pawn Object Reference"))
  (`|ExecutionSequence`
    (:`then_0`
      (cast `/Game/StealthGame/Core/Characters/PlayerCharacter/BP_ThirdPersonCharacterCustom` Pawn
        (:`then`
          (`KismetSystemLibrary.PrintString` "WTF are you doing here?!" true true (struct :`R` 1.0 :`G` 0.005637 :`A` 1.0))
          ;[0.3038 1 0.385 0.5] remember to turn this back on
          (set `self.bPlayerVisible` true))
        (:`CastFailed`
          (set `self.bPlayerVisible` false))))
    (:`then_1`
      (`KismetSystemLibrary.RetriggerableDelay` 1.0)
      (set `self.bPlayerVisible` false)
      (`KismetSystemLibrary.PrintString` "Must have been the wind..." true true (struct :`G` 1.0 :`B` 0.377945 :`A` 1.0)))))

(event `ChasePlayer`
  (`self.UpdateWalkSpeed` 600.0)
  (set `self.bCanMove` false)
  (`|AIMoveTo` self (0.0 0.0 0.0) (`GameplayStatics.GetPlayerCharacter` 0) 100.0
    (:`then`
      (`KismetSystemLibrary.PrintString` "Bonk")
      (set `self.bCanMove` true))))

(event `PatrolRandom`
  (`self.UpdateWalkSpeed` 200.0)
  (set `self.bCanMove` false)
  (`|AIMoveTo` self (`NavigationSystemV1.K2_GetRandomReachablePointInRadius` (`self.K2_GetActorLocation`) 2000.0 null null) null 0.0
    (:`OnSuccess`
      _)
    (:`OnFail`
      _))
  (`KismetSystemLibrary.Delay` 3.0)
  (set `self.bCanMove` true))

(event `MoveToNextPatrolPoint`
  (`self.UpdateWalkSpeed` 200.0)
  (set `self.bCanMove` false)
  (`|AIMoveTo` self (0.0 0.0 0.0) (`|GetArrayItem` (`self.TargetsPoints`) (`self.PatrolTargetPointIndex`))
    (:`OnSuccess`
      (`self.SetNextPointIndex`)
      (`KismetSystemLibrary.Delay` 0.2)
      (set `self.bCanMove` true))
    (:`OnFail`
      (`KismetSystemLibrary.Delay` 0.2)
      (set `self.bCanMove` true))))

(event `SetNextPointIndex`
  (set `self.PatrolTargetPointIndex` (mod (+ (`self.PatrolTargetPointIndex`) 1) (`KismetArrayLibrary.Array_Length` (`self.TargetsPoints`)))))

(fn `UpdateWalkSpeed`
  (params (`Max Walk Speed` :type "Float (double-precision)"))
  (set `CharacterMovementComponent.MaxWalkSpeed` `Max Walk Speed` (`self.CharacterMovement`)))

(fn `UserConstructionScript`)