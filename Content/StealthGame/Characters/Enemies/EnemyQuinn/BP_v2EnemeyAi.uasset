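; Stealth enemy character that patrols target points, chases the player on sight and sends them back to a checkpoint with a melee hit.
; Tick drives AIMoveTo patrol or chase using CanMove and PlayerVisible, with a retriggerable delay clearing sight.
; Hearing noise diverts it to the distraction item's landing point.
; An attack montage notify runs a hand-socket sphere trace, re-arming until the player is hit.
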(event `self.ReceiveBeginPlay`
  (`|ExecutionSequence`
    (:`then_0`
      (bind _returnvalue (`GameplayStatics.GetActorOfClass` "/Game/StealthGame/Gadgets/NoiseMakers/BP_DistractionItemPawn.BP_DistractionItemPawn_C"))
      (set `self.DistractionItemRef` _returnvalue))))

(event `self.ReceiveTick`
  (params (DeltaSeconds :type "Float (single-precision)"))
  (bind _bplayervisible (`self.bPlayerVisible`))
  (if (`self.bCanMove`)
    (if _bplayervisible
      (`self.ChasePlayer`)
      (elif (`self.bTargetPointBoolean`)
        (`self.MoveToNextPatrolPoint`)))
    (elif _bplayervisible
      (`self.ChasePlayer`))))

(event `self.PawnSensing.OnSeePawn`
  (params (Pawn :type "Pawn Object Reference"))
  ; pawn sensing
  (`|ExecutionSequence`
    (:`then_0`
      (cast `/Game/StealthGame/Core/Characters/PlayerCharacter/BP_ThirdPersonCharacterCustom` Pawn
        (:`then`
          (`KismetSystemLibrary.PrintString` "WTF are you doing here?!" true true (struct :`R` 1.0 :`G` 0.005637 :`A` 1.0))
          ;;[0.3038 1 0.385 0.5] remember to turn this back on
          (set `self.bPlayerVisible` true))
        (:`CastFailed`
          (set `self.bPlayerVisible` false))))
    (:`then_1`
      (`KismetSystemLibrary.RetriggerableDelay` 1.0)
      (set `self.bPlayerVisible` false)
      (`KismetSystemLibrary.PrintString` "Must have been the wind..." true true (struct :`G` 1.0 :`B` 0.377945 :`A` 1.0)))))

(event `ChasePlayer`
  (`|ExecutionSequence`
    (:`then_0`
      (`/Engine/EditorBlueprintResources/StandardMacros.DoOnce` false
        (:`Completed`
          (`GameplayStatics.PlaySound2D` "/Game/StealthGame/Gadgets/NoiseMakers/SW_HEYYYY.SW_HEYYYY" 3.0 1.5 0.0 null null))))
    (:`then_1`
      (`self.UpdateWalkSpeed` 500.0)
      (set `self.bCanMove` false)
      (`|AIMoveTo` self (0.0 0.0 0.0) (`GameplayStatics.GetPlayerCharacter` 0) 100.0
        (:`then`
          (`KismetSystemLibrary.PrintString` "Bonk")
          (`self.Attack`)
          (set `self.bCanMove` true))))))

(event `Attack`
  (bind _returnvalue (`SceneComponent.GetSocketLocation` (`self.Mesh`) "hand_r"))
  ;[0.15 0.1407 0.04319 0.5] Bonk
  (`/Engine/EditorBlueprintResources/StandardMacros.DoOnce` false :!label _label ; Only Reset Attack on miss.
    (:`Completed`
      (bind _notifyname (`|PlayMontage` (`self.Mesh`) "/Game/StealthGame/Characters/Enemies/EnemyQuinn/RTG_EnemyAnimations/AM_MIXAMOA_EnemyAttack_Montage.AM_MIXAMOA_EnemyAttack_Montage") ; Play the AM_Attack_01
        (:`OnCompleted`
          (if (`self.bHostile`)
            (`self.ResetAttack`)))
        (:`OnNotifyBegin`
          (switch `name` _notifyname ; Pick the proper attack type(standard when there is more than one type of attack)
            (:`AttackDamage`
              (`KismetSystemLibrary.PrintString` "I'm attacking!")
              (bind (_outhits _returnvalue_2) (`KismetSystemLibrary.SphereTraceMultiForObjects` _returnvalue (+ _returnvalue (* (`self.GetActorForwardVector`) (`self.Melee Trace Distance`))) (`self.Melee Trace Radius`) (`|MakeArray` "ObjectTypeQuery3" :!type "EObjectTypeQuery Enum"))) ; Trace forward from hand socket.
              (if _returnvalue_2
                (for _array_element _outhits
                  (bind _asbp_third_person_character_custom (cast `/Game/StealthGame/Core/Characters/PlayerCharacter/BP_ThirdPersonCharacterCustom` (`.HitActor` (`GameplayStatics.BreakHitResult` _array_element))))
                  (`/Game/StealthGame/Core/Characters/PlayerCharacter/BP_ThirdPersonCharacterCustom.Load Checkpoint` _asbp_third_person_character_custom)
                  (set `self.bHostile` false) ; ...and stop attacking...
                )))))))))

(event `ResetAttack`
  ;[0.15 0.1407 0.04319 0.5] Bonk
  (goto _label :!via `Reset`))

(event `PatrolRandom`
  ;[0.15 0.1407 0.04319 0.5] Bonk
  (`self.UpdateWalkSpeed` 100.0)
  (set `self.bCanMove` false)
  (`|AIMoveTo` self (`NavigationSystemV1.K2_GetRandomReachablePointInRadius` (`self.K2_GetActorLocation`) 2000.0 null null) null 0.0
    (:`OnSuccess`
      (`KismetSystemLibrary.Delay` 3.0)
      (set `self.bCanMove` true))))

(event `MoveToNextPatrolPoint`
  (`self.UpdateWalkSpeed` 100.0)
  (set `self.bCanMove` false)
  (`|AIMoveTo` self (0.0 0.0 0.0) (`|GetArrayItem` (`self.TargetsPoints`) (`self.PatrolTargetPointIndex`))
    (:`OnSuccess`
      (`self.SetNextPointIndex`)
      (`KismetSystemLibrary.Delay` 0.2)
      (set `self.bCanMove` true))))

(event `SetNextPointIndex`
  ; Comment
  (set `self.PatrolTargetPointIndex` (mod (+ (`self.PatrolTargetPointIndex`) 1) (`KismetArrayLibrary.Array_Length` (`self.TargetsPoints`)))))

(event `self.KillZone (CollisionCylinder).OnComponentBeginOverlap`
  (params (OverlappedComponent :type "PrimitiveComponent Object Reference") (OtherActor :type "Actor Object Reference") (OtherComp :type "PrimitiveComponent Object Reference") (OtherBodyIndex :type Integer) (bFromSweep :type Boolean) (SweepResult :type "HitResult Structure (by ref)"))
  ; Killzone (send back to checkpoint spawn
)

(event `self.PawnSensing.OnHearNoise`
  (params (Instigator :type "Pawn Object Reference") (Location :type "Vector Structure (by ref)") (Volume :type "Float (single-precision)"))
  ; Comment
  (`self.UpdateWalkSpeed` 200.0)
  (set `self.bCanMove` false)
  (`|AIMoveTo` self (`/Game/StealthGame/Gadgets/NoiseMakers/BP_DistractionItemPawn.PathEndLocation` (`self.DistractionItemRef`)) null 100.0
    (:`OnSuccess`
      (`KismetSystemLibrary.Delay` 12.0)
      (set `self.bCanMove` true))))

(fn `UpdateWalkSpeed`
  (params (`Max Walk Speed` :type "Float (double-precision)"))
  (set `CharacterMovementComponent.MaxWalkSpeed` `Max Walk Speed` (`self.CharacterMovement`)))

(fn `UserConstructionScript`)