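; BP_UnlockedDoor is an interactable door in the stealth game that swings open and closed.
; Its OpenDoor event stores the open state and picks the swing side from the dot product of the character's and door's forward vectors, so the door opens away from the character.
; The DoorOpen timeline lerps the door mesh's relative yaw to that angle, and closing reverses the timeline from its end.
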(event `OpenDoor`
  (params (Open :type Boolean) (`Char Forward Vector` :type "Vector Structure"))
  (bind _output_get (set `self.IsOpen` Open))
  (if _output_get
    (set `self.Rotation` (select `bool` (> (`KismetMathLibrary.Dot_VectorVector` `Char Forward Vector` (`self.GetActorForwardVector`)) 0.0) :`false` -90.0 :`true` 90.0))
    (bind (_direction _door_open) (`Timeline|Door Open` :!label _label)
      (:`Update`
        (`SceneComponent.K2_SetRelativeRotation` (`self.SM_Door`) (`KismetMathLibrary.MakeRotator` 0.0 0.0 (`KismetMathLibrary.Lerp` 0.0 (`self.Rotation`) _door_open)) false false)))
    (else
      (goto _label :!via `ReverseFromEnd`))))

(fn `UserConstructionScript`)