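; Stealth locker placeable that the player character can hide in and leave with the Interact input.
; A box overlap with the custom third-person character enables input and opens a gate for Interact; leaving disables both.
; ToggleHide flips the character's visibility, collision and movement, blending the camera between locker and character.
; A door timeline plays alongside, but its yaw lerp has identical endpoints; older door-swing logic is left unconnected.
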(event `Hide`)

(event `Unhide`)

(event `InputAction|Interact`
  (params (Key :type "Key Structure"))
  (:`Pressed`
    (`/Engine/EditorBlueprintResources/StandardMacros.Gate` true :!label _label
      (:`Exit`
        (`|ExecutionSequence`
          (:`then_0`
            (`self.ToggleHide`)
            (`KismetSystemLibrary.Delay` 0.2)
            (`self.EnableInput` (`GameplayStatics.GetPlayerController` 0) :!label _label_2)
            (goto _label :!via `Open`))
          (:`then_1`
            (bind (_direction _openclose) (`Timeline|OpenCloseDoor`)
              (:`Update`
                (`SceneComponent.K2_SetRelativeRotation` (`self.SM_locker_0001_door`) (`KismetMathLibrary.MakeRotator` 0.0 0.0 (`KismetMathLibrary.Lerp` 0.0 0.0 _openclose)) false false)))))))))

(event `self.Box.OnComponentBeginOverlap`
  (params (OverlappedComponent :type "PrimitiveComponent Object Reference") (OtherActor :type "Actor Object Reference") (OtherComp :type "PrimitiveComponent Object Reference") (OtherBodyIndex :type Integer) (bFromSweep :type Boolean) (SweepResult :type "HitResult Structure (by ref)"))
  (bind _asbp_third_person_character_custom (cast `/Game/StealthGame/Core/Characters/PlayerCharacter/BP_ThirdPersonCharacterCustom` OtherActor))
  (set `self.As BP Third Person Character Custom` _asbp_third_person_character_custom)
  (goto _label_2))

(event `self.Box.OnComponentEndOverlap`
  (params (OverlappedComponent :type "PrimitiveComponent Object Reference") (OtherActor :type "Actor Object Reference") (OtherComp :type "PrimitiveComponent Object Reference") (OtherBodyIndex :type Integer))
  (bind _asbp_third_person_character_custom (cast `/Game/StealthGame/Core/Characters/PlayerCharacter/BP_ThirdPersonCharacterCustom` OtherActor))
  (set `self.As BP Third Person Character Custom` _asbp_third_person_character_custom)
  (`self.DisableInput` (`GameplayStatics.GetPlayerController` 0))
  (goto _label :!via `Close`))

(event `Key|E`
  (params (Key :type "Key Structure")))

(fn `ToggleHide`
  (bind _as_bp_third_person_character_custom (`self.As BP Third Person Character Custom`))
  (bind _as_bp_third_person_character_custom_2 (`self.As BP Third Person Character Custom`))
  (if (`self.IsHide?`)
    (set `self.IsHide?` false)
    ; Not hidden
    (`self.SetActorEnableCollision` _as_bp_third_person_character_custom true)
    (`self.SetActorHiddenInGame` _as_bp_third_person_character_custom false)
    (`CharacterMovementComponent.SetMovementMode` (`Character.CharacterMovement` _as_bp_third_person_character_custom) "MOVE_Walking" 0)
    (`PlayerController.SetViewTargetWithBlend` (`GameplayStatics.GetPlayerController` 0) (`self.As BP Third Person Character Custom`) 0.5 "VTBlend_Linear" 0.0 false)
    (else
      (set `self.IsHide?` true)
      ; Hidden
      (`self.SetActorEnableCollision` _as_bp_third_person_character_custom_2 false)
      (`self.SetActorHiddenInGame` _as_bp_third_person_character_custom_2 true)
      (`CharacterMovementComponent.DisableMovement` (`Character.CharacterMovement` _as_bp_third_person_character_custom_2))
      (`PlayerController.SetViewTargetWithBlend` (`GameplayStatics.GetPlayerController` 0) self 0.5 "VTBlend_Linear" 0.0 false))))

(fn `UserConstructionScript`)