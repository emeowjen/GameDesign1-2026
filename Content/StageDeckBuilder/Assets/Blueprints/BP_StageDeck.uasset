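; Modular stage deck actor that builds a deck with legs, optional border and four toggleable railings from a chosen shape.
; The construction script looks up the shape's row in DT_DeckShape, assigns meshes and offsets, then applies materials.
; A height value drives leg scale, deck elevation and border scale, with border scale clamped to near zero.
; The SetDeck event repeats the same rebuild outside construction, using a duplicate railing visibility function.
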(event `SetDeck`
  (bind _railing_right (`self.Railing Right`))
  (bind _railing_back (`self.Railing Back`))
  (bind _railing_front (`self.Railing Front`))
  (bind _railing_left (`self.Railing Left`))
  (bind _railing_lx (`self.Railing_LX`))
  (bind _railing_fx (`self.Railing_FX`))
  (bind _railing_bx (`self.Railing_BX`))
  (bind _railing_rx (`self.Railing_RX`))
  (bind _deckborder (`self.DeckBorder`))
  (bind _has_border_ (`self.Has Border?`))
  (bind _returnvalue (`|GetDataTableRow` "/Game/StageDeckBuilder/Assets/Blueprints/DT_DeckShape.DT_DeckShape" (`.List Name` (`self.Deck List` (`self.Deck Shape`))))
    (:`then`
      (set `self.ShapeDataLIst` _returnvalue)
      (`self.SetupDeck`)
      (`self.Design`)
      (bind (_height_out _deck_z_out _border_z_out) (`/Game/StageDeckBuilder/Assets/Blueprints/BP_Functions.ScaleValues` (`self.Height`)))
      (`SceneComponent.SetRelativeScale3D` (`self.DeckLeg`) (`KismetMathLibrary.MakeVector` 1.0 1.0 _height_out))
      (`SceneComponent.K2_SetRelativeLocation` (`self.StageDeck`) (`KismetMathLibrary.MakeVector` 0.0 0.0 _deck_z_out) false false)
      (`SceneComponent.SetVisibility` _deckborder _has_border_ false)
      (`SceneComponent.SetHiddenInGame` _deckborder (not _has_border_) false)
      (`SceneComponent.SetVisibility` _railing_lx _railing_left false)
      (`SceneComponent.SetHiddenInGame` _railing_lx (not _railing_left) false)
      (`SceneComponent.SetVisibility` _railing_fx _railing_front false)
      (`SceneComponent.SetHiddenInGame` _railing_fx (not _railing_front) false)
      (`SceneComponent.SetVisibility` _railing_bx _railing_back false)
      (`SceneComponent.SetHiddenInGame` _railing_bx (not _railing_back) false)
      (`SceneComponent.SetVisibility` _railing_rx _railing_right false)
      (`SceneComponent.SetHiddenInGame` _railing_rx (not _railing_right) false)
      (if (>= _border_z_out 0.001)
        (`SceneComponent.SetRelativeScale3D` _deckborder (`KismetMathLibrary.MakeVector` 1.0 1.0 _border_z_out))
        (else
          (`SceneComponent.SetRelativeScale3D` _deckborder (1.0 1.0 0.0001)))))))

(fn `SetupDeck`
  (bind (_shapedatalist_deck _shapedatalist_legs _shapedatalist_border _shapedatalist_railinglx _shapedatalist_railingrx _shapedatalist_railingfx _shapedatalist_railingbx _shapedatalist_railinglxyoffset _shapedatalist_railingrxyoffset _shapedatalist_railingfxxoffset _shapedatalist_railingbxxoffset _shapedatalist_borderoffset _shapedatalist_borderrot) (break `/Game/StageDeckBuilder/Assets/Blueprints/STRU_DeckSetups` (`self.ShapeDataLIst`)))
  (bind _deckborder (`self.DeckBorder`))
  (bind _railing_lx (`self.Railing_LX`))
  (bind _railing_fx (`self.Railing_FX`))
  (bind _railing_bx (`self.Railing_BX`))
  (bind _railing_rx (`self.Railing_RX`))
  (`StaticMeshComponent.SetStaticMesh` (`self.StageDeck`) _shapedatalist_deck)
  (`StaticMeshComponent.SetStaticMesh` (`self.DeckLeg`) _shapedatalist_legs)
  (`StaticMeshComponent.SetStaticMesh` _deckborder _shapedatalist_border)
  (`SceneComponent.K2_SetRelativeLocationAndRotation` _deckborder (`KismetMathLibrary.MakeVector` (.x _shapedatalist_borderoffset) (.y _shapedatalist_borderoffset) (.z _shapedatalist_borderoffset)) _shapedatalist_borderrot false false)
  (`StaticMeshComponent.SetStaticMesh` _railing_lx _shapedatalist_railinglx)
  (`SceneComponent.K2_SetRelativeLocationAndRotation` :`self` _railing_lx :`NewLocation` (`KismetMathLibrary.MakeVector` (.x _shapedatalist_railinglxyoffset) (.y _shapedatalist_railinglxyoffset) (.z _shapedatalist_railinglxyoffset)))
  (`StaticMeshComponent.SetStaticMesh` _railing_rx _shapedatalist_railingrx)
  (`SceneComponent.K2_SetRelativeLocationAndRotation` :`self` _railing_rx :`NewLocation` (`KismetMathLibrary.MakeVector` (.x _shapedatalist_railingrxyoffset) (.y _shapedatalist_railingrxyoffset) (.z _shapedatalist_railingrxyoffset)))
  (`StaticMeshComponent.SetStaticMesh` _railing_fx _shapedatalist_railingfx)
  (`SceneComponent.K2_SetRelativeLocationAndRotation` _railing_fx (`KismetMathLibrary.MakeVector` (.x _shapedatalist_railingfxxoffset) (.y _shapedatalist_railingfxxoffset) (.z _shapedatalist_railingfxxoffset)) (struct :`Yaw` 90.0) false false)
  (`StaticMeshComponent.SetStaticMesh` _railing_bx _shapedatalist_railingbx)
  (`SceneComponent.K2_SetRelativeLocationAndRotation` _railing_bx (`KismetMathLibrary.MakeVector` (.x _shapedatalist_railingbxxoffset) (.y _shapedatalist_railingbxxoffset) (.z _shapedatalist_railingbxxoffset)) (struct :`Yaw` 90.0) false false)
  (return))

(fn `UserConstructionScript`
  (bind _railing_right (`self.Railing Right`))
  (bind _railing_back (`self.Railing Back`))
  (bind _railing_front (`self.Railing Front`))
  (bind _railing_left (`self.Railing Left`))
  (bind _railing_lx (`self.Railing_LX`))
  (bind _railing_fx (`self.Railing_FX`))
  (bind _railing_bx (`self.Railing_BX`))
  (bind _railing_rx (`self.Railing_RX`))
  (bind _deckborder (`self.DeckBorder`))
  (bind _has_border_ (`self.Has Border?`))
  (bind _returnvalue (`|GetDataTableRow` "/Game/StageDeckBuilder/Assets/Blueprints/DT_DeckShape.DT_DeckShape" (`.List Name` (`self.Deck List` (`self.Deck Shape`))))
    (:`then`
      (set `self.ShapeDataLIst` _returnvalue)
      (`self.SetupDeck`)
      (`self.Design`)
      (bind (_height_out _deck_z_out _border_z_out) (`/Game/StageDeckBuilder/Assets/Blueprints/BP_Functions.ScaleValues` (`self.Height`)))
      (`SceneComponent.SetRelativeScale3D` (`self.DeckLeg`) (`KismetMathLibrary.MakeVector` 1.0 1.0 _height_out))
      (`SceneComponent.K2_SetRelativeLocation` (`self.StageDeck`) (`KismetMathLibrary.MakeVector` 0.0 0.0 _deck_z_out) false false)
      (`SceneComponent.SetVisibility` _deckborder _has_border_ false)
      (`SceneComponent.SetHiddenInGame` _deckborder (not _has_border_) false)
      (`SceneComponent.SetVisibility` _railing_lx _railing_left false)
      (`SceneComponent.SetHiddenInGame` _railing_lx (not _railing_left) false)
      (`SceneComponent.SetVisibility` _railing_fx _railing_front false)
      (`SceneComponent.SetHiddenInGame` _railing_fx (not _railing_front) false)
      (`SceneComponent.SetVisibility` _railing_bx _railing_back false)
      (`SceneComponent.SetHiddenInGame` _railing_bx (not _railing_back) false)
      (`SceneComponent.SetVisibility` _railing_rx _railing_right false)
      (`SceneComponent.SetHiddenInGame` _railing_rx (not _railing_right) false)
      (if (>= _border_z_out 0.001)
        (`SceneComponent.SetRelativeScale3D` _deckborder (`KismetMathLibrary.MakeVector` 1.0 1.0 _border_z_out))
        (else
          (`SceneComponent.SetRelativeScale3D` _deckborder (1.0 1.0 0.0001)))))))