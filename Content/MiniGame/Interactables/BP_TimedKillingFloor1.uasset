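; BP_TimedKillingFloor1 is a minigame hazard floor that periodically appears and disappears.
; A looping timer started on BeginPlay toggles the Cube's visibility and collision together every 1.5 seconds.
; When a BP_ThirdPersonCharacterCustom overlaps the Cube, it calls LoadCheckpoint on that character, sending it back to its checkpoint.
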(event `self.Cube.OnComponentBeginOverlap`
  (params (OverlappedComponent :type "PrimitiveComponent Object Reference") (OtherActor :type "Actor Object Reference") (OtherComp :type "PrimitiveComponent Object Reference") (OtherBodyIndex :type Integer) (bFromSweep :type Boolean) (SweepResult :type "HitResult Structure (by ref)"))
  (bind _asbp_third_person_character_custom (cast `/Game/StealthGame/Core/Characters/PlayerCharacter/BP_ThirdPersonCharacterCustom` OtherActor))
  (`/Game/StealthGame/Core/Characters/PlayerCharacter/BP_ThirdPersonCharacterCustom.Load Checkpoint` _asbp_third_person_character_custom))

(event `self.ReceiveBeginPlay`
  ; Looping visibility
  (`KismetSystemLibrary.K2_SetTimerDelegate` (delegate `EventManagePlatform`) 1.5 true))

(event `EventManagePlatform`
  ; Looping visibility
  (if (`SceneComponent.bVisible` (`self.Cube`))
    (`SceneComponent.SetVisibility` (`self.Cube`) false false)
    (`PrimitiveComponent.SetCollisionEnabled` (`self.Cube`) "NoCollision")
    (else
      (`SceneComponent.SetVisibility` (`self.Cube`) true false)
      (`PrimitiveComponent.SetCollisionEnabled` (`self.Cube`) "QueryAndPhysics"))))

(fn `UserConstructionScript`)